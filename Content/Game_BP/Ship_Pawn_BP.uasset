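; Player ship pawn that drives the thrusters of a SpaceCraft held in a child actor component.
; The Thrust axis copies the pawn's ThrustStrength to four physics thrusters and activates them only at exactly full input, otherwise deactivating them.
; Roll, Pitch and Yaw inputs have no logic yet; Tick prints their values and Thrust for debugging.
; BeginPlay sets the player controller as the camera manager's owner.
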(event `self.ReceiveBeginPlay`
  (`self.SetOwner` (`GameplayStatics.GetPlayerCameraManager` 0) (`GameplayStatics.GetPlayerController` 0)))

(event `InputAxis|Thrust`
  (params (AxisValue :type "Float (single-precision)"))
  (bind _thrust_strength (`self.Thrust Strength`))
  (bind _asspace_craft (cast `/Game/Core/SpaceCraft` (`ChildActorComponent.ChildActor` (`self.SpaceCraft`))))
  (if (== AxisValue 1.0)
    (bind _physicsthruster (`/Game/Core/SpaceCraft.PhysicsThruster` _asspace_craft))
    (set `PhysicsThrusterComponent.ThrustStrength` _thrust_strength _physicsthruster)
    (bind _physicsthruster1 (`/Game/Core/SpaceCraft.PhysicsThruster1` _asspace_craft))
    (set `PhysicsThrusterComponent.ThrustStrength` _thrust_strength _physicsthruster1)
    (set `PhysicsThrusterComponent.ThrustStrength` _thrust_strength (`/Game/Core/SpaceCraft.PhysicsThruster2` _asspace_craft))
    (set `PhysicsThrusterComponent.ThrustStrength` _thrust_strength (`/Game/Core/SpaceCraft.PhysicsThruster3` _asspace_craft))
    (`ActorComponent.Activate` _physicsthruster1 false)
    (`ActorComponent.Activate` (`/Game/Core/SpaceCraft.PhysicsThruster2` _asspace_craft) false)
    (`ActorComponent.Activate` _physicsthruster false)
    (`ActorComponent.Activate` (`/Game/Core/SpaceCraft.PhysicsThruster3` _asspace_craft) false)
    (else
      (`ActorComponent.Deactivate` _physicsthruster)
      (`ActorComponent.Deactivate` _physicsthruster1)
      (`ActorComponent.Deactivate` (`/Game/Core/SpaceCraft.PhysicsThruster2` _asspace_craft))
      (`ActorComponent.Deactivate` (`/Game/Core/SpaceCraft.PhysicsThruster3` _asspace_craft)))))

(event `self.ReceiveTick`
  (params (DeltaSeconds :type "Float (single-precision)"))
  (`|ExecutionSequence`
    (:`then_0`
      (`KismetSystemLibrary.PrintString` (`KismetStringLibrary.Concat_StrStr` "Roll:  " (`KismetStringLibrary.Conv_DoubleToString` (`self.GetInputAxisValue`)) "Pitch: " (`KismetStringLibrary.Conv_DoubleToString` (`self.GetInputAxisValue`)) "Yaw: " (`KismetStringLibrary.Conv_DoubleToString` (`self.GetInputAxisValue`)) "Thrust: " (`KismetStringLibrary.Conv_DoubleToString` (`self.GetInputAxisValue`))) true true (struct :`G` 0.66 :`B` 1.0 :`A` 1.0) 0.1))))

(event `InputAxis|Roll`
  (params (AxisValue :type "Float (single-precision)")))

(event `InputAxis|Pitch`
  (params (AxisValue :type "Float (single-precision)")))

(event `InputAxis|Yaw`
  (params (AxisValue :type "Float (single-precision)")))

(fn `UserConstructionScript`)