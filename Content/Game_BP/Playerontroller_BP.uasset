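; Player controller Blueprint that feeds thruster power input to the referenced TrainPL object.
; On a non-zero "Thruster power" axis value, it checks that TrainPL is valid, then adds the scaled input to its FL0, FR1, RL2 and RR3 values equally.
; The adjustment accumulates with each input event, with no clamping or delta-time scaling here.
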(event `InputAxis|Thruster power`
  (params (AxisValue :type "Float (single-precision)"))
  (bind _returnvalue (* AxisValue 0.05))
  (bind _trainpl (`self.TrainPL`))
  (if (!= AxisValue 0.0)
    (`/Engine/EditorBlueprintResources/StandardMacros.IsValid` _trainpl
      (:`Is Valid`
        (set `/Game/8Engines_Actot_BP.FL0` (+ _returnvalue (`/Game/8Engines_Actot_BP.FL0` _trainpl)) _trainpl)
        (set `/Game/8Engines_Actot_BP.FR1` (+ _returnvalue (`/Game/8Engines_Actot_BP.FR1` _trainpl)) _trainpl)
        (set `/Game/8Engines_Actot_BP.RL2` (+ _returnvalue (`/Game/8Engines_Actot_BP.RL2` _trainpl)) _trainpl)
        (set `/Game/8Engines_Actot_BP.RR3` (+ _returnvalue (`/Game/8Engines_Actot_BP.RR3` _trainpl)) _trainpl)))))

(fn `UserConstructionScript`)