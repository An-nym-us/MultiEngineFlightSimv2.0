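; Player-controlled Pelican aircraft prototype flown with physics thrusters.
; BeginPlay spawns a Flightinterface actor and activates four corner thrusters, which an input toggles; Pitch input fires two rear thrusters.
; Thrust Up/Down should adjust shared strength, but their contradictory axis checks never pass.
; Tick runs an unused ground trace, empty update stubs, and a center-of-mass marker positioned by the offset from the body's origin.
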(event `UpdateMovingThruster`
  (params (Target :type "SceneComponent Object Reference")))

(event `self.ReceiveBeginPlay`
  (`|ExecutionSequence`
    (:`then_0`
      (bind _returnvalue (`|SpawnActorFromClass` "/Script/MultiEngineFlightSim.flightinterface" (`self.GetTransform`) "AlwaysSpawn" "OverrideRootScale" self self))
      (`/Engine/EditorBlueprintResources/StandardMacros.IsValid` _returnvalue
        (:`Is Valid`
          (set `self.Interface Object` _returnvalue))))
    (:`then_1`
      (`ActorComponent.Activate` (`self.PhysicsThrusterFL`) false :!label _label)
      (`ActorComponent.Activate` (`self.PhysicsThrusterRL`) false)
      (`ActorComponent.Activate` (`self.PhysicsThrusterFR`) false)
      (`ActorComponent.Activate` (`self.PhysicsThrusterRR`) false)
      (`KismetSystemLibrary.PrintString` (`KismetStringLibrary.Conv_BoolToString` (not (stale `InputAction|Activate Thrusters` _isa))) true true (struct :`R` 1.0 :`G` 0.160329 :`A` 1.0) :!label _label_2))))

(event `InputAction|Activate Thrusters`
  (params (Key :type "Key Structure"))
  (:`Pressed`
    (bind _isa (`/Engine/EditorBlueprintResources/StandardMacros.FlipFlop`)
      (:`A`
        (`ActorComponent.Deactivate` (`self.PhysicsThrusterFL`))
        (`ActorComponent.Deactivate` (`self.PhysicsThrusterRL`))
        (`ActorComponent.Deactivate` (`self.PhysicsThrusterFR`))
        (`ActorComponent.Deactivate` (`self.PhysicsThrusterRR`))
        (goto _label_2))
      (:`B`
        (goto _label)))))

(event `InputAxis|Thrust Down`
  (params (AxisValue :type "Float (single-precision)"))
  (bind _returnvalue (* (`self.Thrust Strength`) 1.0))
  (if (and (== AxisValue -1.0) (== (stale `InputAxis|Thrust Up` AxisValue) 0.0))
    (set `self.Thrust Strength` (+ (* AxisValue 100000.0) (`self.Thrust Strength`)))
    (if true :!label _label_3
      (set `PhysicsThrusterComponent.ThrustStrength` _returnvalue (`self.PhysicsThrusterFL`))
      (set `PhysicsThrusterComponent.ThrustStrength` _returnvalue (`self.PhysicsThrusterRL`))
      (set `PhysicsThrusterComponent.ThrustStrength` _returnvalue (`self.PhysicsThrusterFR`))
      (bind _output_get (set `PhysicsThrusterComponent.ThrustStrength` _returnvalue (`self.PhysicsThrusterRR`)))
      (`KismetSystemLibrary.PrintString` (`KismetStringLibrary.Conv_DoubleToString` _output_get) true true (struct :`G` 0.66 :`B` 1.0 :`A` 1.0) 0.1))))

(event `InputAxis|Thrust Up`
  (params (AxisValue :type "Float (single-precision)"))
  (if (and (== AxisValue 1.0) (== (stale `InputAxis|Thrust Down` AxisValue) 0.0))
    (set `self.Thrust Strength` (+ (* AxisValue 100000.0) (`self.Thrust Strength`)))
    (goto _label_3)))

(event `InputAxis|Pitch`
  (params (AxisValue :type "Float (single-precision)"))
  (bind _physicsthrusterrear_left (`self.PhysicsThrusterRear Left`))
  (bind _thrust_strength_0 (`self.Thrust Strength_0`))
  (if (!= AxisValue 0.0)
    (set `PhysicsThrusterComponent.ThrustStrength` _thrust_strength_0 _physicsthrusterrear_left)
    (set `PhysicsThrusterComponent.ThrustStrength` _thrust_strength_0 (`self.PhysicsThruster Rear Right`))
    (`ActorComponent.Activate` _physicsthrusterrear_left false)
    (`ActorComponent.Activate` (`self.PhysicsThruster Rear Right`) false)
    (else
      (`ActorComponent.Deactivate` _physicsthrusterrear_left)
      (`ActorComponent.Deactivate` (`self.PhysicsThruster Rear Right`)))))

(event `self.ReceiveTick`
  (params (DeltaSeconds :type "Float (single-precision)"))
  (`|ExecutionSequence`
    (:`then_0`
      (`self.Current Elevation Off Ground`))
    (:`then_1`
      (`self.Current Axis Rotation`))
    (:`then_2`
      (`self.Run System`))
    (:`then_3`
      (`self.see center of mass`))
    (:`then_4`
      (`self.UpdateMovingThruster` null))))

(event `Run System`
  (bind _returnvalue (`SceneComponent.K2_GetComponentLocation` (`self.pellican_Whole_Pelican`)))
  (`/Engine/EditorBlueprintResources/StandardMacros.IsValid` (`self.Interface Object`)
    (:`Is Valid`
      (bind _outhit (`KismetSystemLibrary.LineTraceSingle` _returnvalue (- _returnvalue (0.0 0.0 10000000000.0)) "TraceTypeQuery1")))))

(event `Current Elevation Off Ground`)

(event `see center of mass`
  (bind _pellican_whole_pelican (`self.pellican_Whole_Pelican`))
  (`/Engine/EditorBlueprintResources/StandardMacros.IsValid` (`self.mass view`)
    (:`Is Valid`
      (`self.K2_SetActorLocation` (`self.mass view`) (- (`PrimitiveComponent.GetCenterOfMass` _pellican_whole_pelican "None") (`SceneComponent.K2_GetComponentLocation` _pellican_whole_pelican)) false true))
    (:`Is Not Valid`
      (bind _returnvalue (`|SpawnActorFromClass` "/Game/Game_BP/CubCneterOFMssView.CubCneterOFMssView_C" (`SceneComponent.K2_GetComponentToWorld` (`self.Mesh`)) "Undefined" "OverrideRootScale" null null))
      (set `self.mass view` _returnvalue))))

(event `Current Axis Rotation`)

(fn `UserConstructionScript`)