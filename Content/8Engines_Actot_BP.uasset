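; Ten-thruster physics vehicle that serves as a flight training agent, with episode status and reward held on TargetBP.
; Each tick maps the thruster inputs to clamped thrust strengths and records the cube's pose, velocities and derived linear and angular accelerations.
; Leaving pose limits, completing training or exceeding a reward threshold triggers a DoOnce-guarded reset: randomized X/Z position, zeroed velocities, inputs and reward.
; Fixed-position reset and episode-phase branches are disconnected.
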(event `Update Acceleration`
  (bind _cube (`self.Cube`))
  (bind _output_get (set `self.Velocity` (`SceneComponent.GetComponentVelocity` _cube)))
  (set `self.Acceleration` (/ (- _output_get (`self.Prevous Vel`)) (`GameplayStatics.GetWorldDeltaSeconds`)))
  (set `self.Prevous Vel` (`self.Velocity`))
  (bind _output_get_2 (set `self.Velocity_Degrees` (`PrimitiveComponent.GetPhysicsAngularVelocityInDegrees` _cube "None")))
  (set `self.Acceleration_Degrees` (/ (- _output_get_2 (`self.Previous_Velocity_Degrees`)) (`GameplayStatics.GetWorldDeltaSeconds`)))
  (set `self.Previous_Velocity_Degrees` (`self.Velocity_Degrees`)))

(event `self.ReceiveBeginPlay`)

(event `self.ReceiveTick`
  (params (DeltaSeconds :type "Float (single-precision)"))
  (bind _cube (`self.Cube`))
  (bind _target_bp (`self.Target_BP`))
  (bind _pitch (`self.Pitch`))
  (bind _max_axis_values_pich___ (`self.Max Axis Values Pich +-`))
  (bind _roll (`self.Roll`))
  (bind _yaw (`self.Yaw`))
  (bind _max_axis_values_roll____1 (`self.Max Axis Values Roll +-_1`))
  (bind _max_axis_values_yaw____0 (`self.Max Axis Values Yaw +-_0`))
  (bind _z_axis (`self.Z-Axis`))
  (bind _x_axis (`self.X_Axis`))
  (bind _y_axis (`self.Y_Axis`))
  (bind _max_x_axis (`self.Max X Axis`))
  (bind _max_y_axis_0 (`self.Max Y Axis_0`))
  (bind _max_thrust (`self.Max Thrust`))
  (bind _min_thrust (`self.Min Thrust`))
  (bind _cube_2 (`self.Cube`))
  (bind (_acceleration_x _acceleration_y _acceleration_z) (`KismetMathLibrary.BreakVector` (`self.Acceleration`)))
  (bind (_acceleration_degrees_x _acceleration_degrees_y _acceleration_degrees_z) (`KismetMathLibrary.BreakVector` (`self.Acceleration_Degrees`)))
  (bind (_returnvalue_x _returnvalue_y _returnvalue_z) (`KismetMathLibrary.BreakVector` (`SceneComponent.GetComponentVelocity` _cube_2)))
  (bind (_returnvalue_x_2 _returnvalue_y_2 _returnvalue_z_2) (`KismetMathLibrary.BreakVector` (`PrimitiveComponent.GetPhysicsAngularVelocityInDegrees` _cube_2 "None")))
  (bind _returnvalue (`SceneComponent.K2_GetComponentToWorld` _cube_2))
  (`PrimitiveComponent.WakeAllRigidBodies` (`self.Cube`))
  (`KismetSystemLibrary.DelayUntilNextTick`)
  (`|ExecutionSequence`
    (:`then_0`
      (`self.ClampRangeThruster` (`self.FR1`) _min_thrust _max_thrust 0.0 (`self.PhysicsThrusterFR1`))
      (`self.ClampRangeThruster` (`self.RR3`) _min_thrust _max_thrust 0.0 (`self.PhysicsThrusterRR3`))
      (`self.ClampRangeThruster` (`self.RRFW9`) _min_thrust _max_thrust 0.0 (`self.PhysicsThrusterRRFW9`)))
    (:`then_1`
      (`self.ClampRangeThruster` (`self.FL0`) _min_thrust _max_thrust 0.0 (`self.PhysicsThrusterFL0`))
      (`self.ClampRangeThruster` (`self.RL2`) _min_thrust _max_thrust 0.0 (`self.PhysicsThrusterRL2`))
      (`self.ClampRangeThruster` (`self.RLFW8`) _min_thrust _max_thrust 0.0 (`self.PhysicsThrusterRLFW8`)))
    (:`then_2`
      (`self.Update Acceleration`))
    (:`then_4`
      (`self.ClampRangeThruster` (`self.RRP7`) -1000.0 1000.0 0.0 (`self.PhysicsThrusterRRP7`))
      (`self.ClampRangeThruster` (`self.FRP5`) -1000.0 1000.0 0.0 (`self.PhysicsThrusterFRP5`)))
    (:`then_5`
      (`self.ClampRangeThruster` (`self.LLP6`) -1000.0 1000.0 0.0 (`self.PhysicsThrusterRLP6`))
      (`self.ClampRangeThruster` (`self.FLP4`) -1000.0 1000.0 0.0 (`self.PhysicsThrusterFLP4`)))
    (:`then_6`
      (`|ExecutionSequence`
        (:`then_0`
          (set `self.Pitch` (.pitch (.rotation _returnvalue)))
          (set `self.Roll` (.roll (.rotation _returnvalue)))
          (set `self.Yaw` (.yaw (.rotation _returnvalue)))
          (set `self.X_Axis` (.x (.location _returnvalue)))
          (set `self.Y_Axis` (.y (.location _returnvalue)))
          (set `self.Z-Axis` (.z (.location _returnvalue)))
          (set `self.X-Axis_VEL` _returnvalue_x)
          (set `self.Y-Axis_VEL` _returnvalue_y)
          (set `self.Z-Axis_VEL` _returnvalue_z)
          (set `self.X-Axis_VEL_ANG` _returnvalue_x_2)
          (set `self.Y-Axis_VEL_ANG` _returnvalue_y_2)
          (set `self.Z-Axis_VEL_ANG` _returnvalue_z_2)
          (set `self.X-Axis_Acc` _acceleration_x)
          (set `self.Y-Axis_Acc` _acceleration_y)
          (set `self.Z-Axis_Acc` _acceleration_z)
          (set `self.X-Axis_Acc_Deg` _acceleration_degrees_x)
          (set `self.Y-Axis_Acc_Deg` _acceleration_degrees_y)
          (set `self.Z-Axis_Acc_Deg` _acceleration_degrees_z)
          (if (or (`/Game/Target_Blueprint.Training Complete` _target_bp) (not (and (< _pitch _max_axis_values_pich___) (> _pitch (* _max_axis_values_pich___ -1.0)))) (not (and (< _roll _max_axis_values_roll____1) (> _roll (* _max_axis_values_roll____1 -1.0)))) (not (and (< _yaw _max_axis_values_yaw____0) (> _yaw (* _max_axis_values_yaw____0 -1.0)))) (not (and (< _x_axis _max_x_axis) (> _x_axis (* _max_x_axis -1.0)))) (not (and (< _y_axis _max_y_axis_0) (> _y_axis (* _max_y_axis_0 -1.0)))) (not (and (< _z_axis (`self.Max Z Axis_1`)) (> _z_axis 100.0))) (> (`/Game/Target_Blueprint.Reward` _target_bp) 777.0))
            (`/Engine/EditorBlueprintResources/StandardMacros.DoOnce` false :!label _label
              (:`Completed`
                (set `self.start` false)
                (`/Engine/EditorBlueprintResources/StandardMacros.IncrementInt` (`self.Current Number of resets`)
                  (:`  `
                    (if true
                      ;[1 1 1] Start Createing random variable locations
                      (`KismetSystemLibrary.MoveComponentTo` (`self.Cube`) (`KismetMathLibrary.MakeVector` (`KismetMathLibrary.RandomFloatInRange` -50.0 50.0) 0.0 (`KismetMathLibrary.RandomFloatInRange` 190.0 390.0)) (struct) false false 0.0)
                      (`PrimitiveComponent.SetSimulatePhysics` _cube true)
                      (`PrimitiveComponent.SetPhysicsLinearVelocity` _cube (0.0 0.0 0.0) false "None")
                      (`PrimitiveComponent.SetPhysicsAngularVelocityInDegrees` _cube (0.0 0.0 0.0) false "None")
                      (bind _output_get (set `self.FR1` 0.0))
                      (bind _output_get_2 (set `self.FL0` _output_get))
                      (bind _output_get_3 (set `self.RR3` _output_get_2))
                      (bind _output_get_4 (set `self.RL2` _output_get_3))
                      (bind _output_get_5 (set `self.LLP6` _output_get_4))
                      (bind _output_get_6 (set `self.RRP7` _output_get_5))
                      (bind _output_get_7 (set `self.FLP4` _output_get_6))
                      (bind _output_get_8 (set `self.FRP5` _output_get_7))
                      (bind _output_get_9 (set `self.RRFW9` _output_get_8))
                      (set `self.RLFW8` _output_get_9)
                      (set `/Game/Target_Blueprint.Reward` 0.0 (`self.Target_BP`))
                      (set `self.start` true)
                      (set `/Game/Target_Blueprint.Training Complete` false (`self.Target_BP`))
                      (`self.RESET GATE`))))))))))))

(event `RESET GATE`
  (goto _label :!via `Reset`))

(fn `ClampRangeThruster`
  (params (PercentThrust :type "Float (double-precision)") (`Min Thrust` :type "Float (double-precision)") (`Max Thrust` :type "Float (double-precision)") (`Thruster Step Size` :type "Float (double-precision)") (Thruster :type "PhysicsThrusterComponent Object Reference"))
  (returns (ThrustAmouny :type "Float (double-precision)"))
  (bind _output_get (set `PhysicsThrusterComponent.ThrustStrength` (`KismetMathLibrary.FClamp` (`KismetMathLibrary.Lerp` `Min Thrust` `Max Thrust` (`KismetMathLibrary.NormalizeToRange` PercentThrust -10.0 10.0)) `Min Thrust` `Max Thrust`) Thruster))
  (return _output_get))

(fn `UserConstructionScript`)