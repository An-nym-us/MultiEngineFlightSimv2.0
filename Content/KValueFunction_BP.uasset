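; KValueFunction_BP is a PID controller actor that computes a thrust value from a measured value, target and gains.
; It parses these from the bracketed PIDSendIN string on BeginPlay and each CalledUpdateFromParent, then outputs ThrustOut and echoes gains in PIDSendOut.
; The P term uses the previous error, while I and D use accumulated elapsed time rather than frame delta.
; ResetFornewLeesson zeroes timer, errors, inputs and gains.
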(event `self.ReceiveTick`
  (params (DeltaSeconds :type "Float (single-precision)")))

(event `Reset For new Leesson`
  (set `self.ElapseedTime` 0.0)
  (set `self.P:instanteneousError ` 0.0)
  (set `self.(Integreal Error [Sum])` 0.0)
  (set `self.errorLastCalculation` 0.0)
  (set `self.Y(t) Measured Value` 0.0)
  (set `self.R(t) Desirded Value` 0.0)
  (set `self.K_p` 0.0)
  (set `self.K_i` 0.0)
  (set `self.K_d` 0.0))

(event `self.ReceiveBeginPlay`
  (bind _returnvalue (`KismetStringLibrary.ParseIntoArray` (`KismetStringLibrary.Replace` (`KismetStringLibrary.Replace` (`self.PID_SendIN`) "[") "]") ","))
  (set `self.Y(t) Measured Value` (`KismetStringLibrary.Conv_StringToDouble` (`|GetArrayItem` _returnvalue)) :!label _label)
  (set `self.R(t) Desirded Value` (`KismetStringLibrary.Conv_StringToDouble` (`|GetArrayItem` _returnvalue 1)))
  (set `self.K_p` (`KismetStringLibrary.Conv_StringToDouble` (`|GetArrayItem` _returnvalue 2)))
  (set `self.K_i` (`KismetStringLibrary.Conv_StringToDouble` (`|GetArrayItem` _returnvalue 3)))
  (set `self.K_d` (`KismetStringLibrary.Conv_StringToDouble` (`|GetArrayItem` _returnvalue 4)))
  (set `self.ElapseedTime` (+ (`GameplayStatics.GetWorldDeltaSeconds`) (`self.ElapseedTime`)))
  (`|ExecutionSequence`
    (:`then_0`
      ;[1 1 1] Get Perportional Error
      (set `self.P:instanteneousError ` (- (`self.R(t) Desirded Value`) (`self.Y(t) Measured Value`))))
    (:`then_1`
      ;[1 1 1] sum of all previous errors
      (set `self.(Integreal Error [Sum])` (* (+ (`self.(Integreal Error [Sum])`) (* (`self.P:instanteneousError `) (`self.ElapseedTime`))) 0.1)))
    (:`then_2`
      ;[1 1 1] Derivitive Error
      (set `self.(Derivative Error )` (/ (- (`self.P:instanteneousError `) (`self.errorLastCalculation`)) (`self.ElapseedTime`))))
    (:`then_3`
      (bind _output_get (set `self.U(T) [Percent Add]` (* (+ (* (`self.errorLastCalculation`) (`self.K_p`)) (* (`self.(Integreal Error [Sum])`) (`self.K_i`)) (* (`self.(Derivative Error )`) (`self.K_d`))) 0.1)))
      (set `self.PID_SendOut` (`KismetStringLibrary.Concat_StrStr` (`KismetStringLibrary.Conv_DoubleToString` (`self.K_p`)) "," (`KismetStringLibrary.Conv_DoubleToString` (`self.K_i`)) "," (`KismetStringLibrary.Conv_DoubleToString` (`self.K_d`))))
      (set `self.Thrust Out` _output_get))
    (:`then_4`
      ;[1 1 1 1 12] Save The preveipous calulation for the derivitve claualtion
      (set `self.errorLastCalculation` (`self.P:instanteneousError `)))))

(event `Called Update From Parent`
  (goto _label))

(fn `UserConstructionScript`)